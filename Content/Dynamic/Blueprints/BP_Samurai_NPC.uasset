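; Samurai NPC Blueprint that acts as the computer-controlled attacker in the game's draw phase.
; On BeginPlay it runs the parent's setup, then binds to the game mode's draw-phase-started event.
; When that phase starts, it waits a random delay between AttackDelayMin and AttackDelayMax, then calls Attack, simulating a variable reaction time.
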(event `self.ReceiveBeginPlay`
  (`parent.ReceiveBeginPlay`)
  (add `/Game/Dynamic/Blueprints/GM_Duel.DrawPhaseStarted` (`self.Gamemode`) (delegate `OnDrawPhaseStart`)))

(event `OnDrawPhaseStart`
  (`KismetSystemLibrary.Delay` (`KismetMathLibrary.RandomFloatInRange` (`self.AttackDelayMin`) (`self.AttackDelayMax`)))
  (`self.Attack`))

(fn `UserConstructionScript`
  (`parent.UserConstructionScript`))